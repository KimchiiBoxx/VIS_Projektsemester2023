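; BP_Holografitti_Lotus is a pickup item actor whose mesh is chosen through a variable.
; The construction script applies ItemMeshToPlace to the Item mesh component.
; The PickUp event, commented as following an E press, prints an Origami Crane message despite the Lotus name, then destroys the actor.
; Camera-facing rotation logic for an interaction sign is present but disconnected, so Tick does nothing.
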(event `self.PickUp`
  ;[1 1 1] After press E = destroy Item and print Information
  (`KismetSystemLibrary.PrintString` "You received an Origami Crane.")
  (`self.K2_DestroyActor`))

(event `self.ReceiveTick`
  (params (DeltaSeconds :type "Float (single-precision)"))
  ;[1 1 1] Direction of Interaction Sign
)

(fn `UserConstructionScript`
  (`StaticMeshComponent.SetStaticMesh` (`self.Item`) (`self.ItemMeshToPlace`)))