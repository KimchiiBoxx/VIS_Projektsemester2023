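; BP_Spoon is a spoon pickup that the BP_FP_Fae character collects with the E key.
; Overlapping its trigger enables input and opens a gate for the key press, and leaving closes the gate.
; Both overlap events call EnableInput, so the gate alone limits the pickup range.
; An accepted press sets HasSpoon on the character, plays a sound and destroys the spoon.
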(event `Key|E`
  (params (Key :type "Key Structure"))
  (:`Pressed`
    (`/Engine/EditorBlueprintResources/StandardMacros.Gate` true :!label _label
      (:`Exit`
        (set `/Game/FirstPerson/Blueprints/BP_FP_Fae.HasSpoon?` true (stale `self.Trigger.OnComponentBeginOverlap` _asbp_fp_fae))
        (`GameplayStatics.SpawnSoundAtLocation` "/Game/03_Sound/Interaction/SC_TakeWithMe_Cue.SC_TakeWithMe_Cue" (0.0 0.0 0.0) (struct) 1.0 1.0 0.0 null null)
        (`self.K2_DestroyActor`)))))

(event `self.Trigger.OnComponentBeginOverlap`
  (params (OverlappedComponent :type "PrimitiveComponent Object Reference") (OtherActor :type "Actor Object Reference") (OtherComp :type "PrimitiveComponent Object Reference") (OtherBodyIndex :type Integer) (bFromSweep :type Boolean) (SweepResult :type "HitResult Structure (by ref)"))
  (bind _asbp_fp_fae (cast `/Game/FirstPerson/Blueprints/BP_FP_Fae` OtherActor))
  (`self.EnableInput` (`GameplayStatics.GetPlayerController` 0))
  (goto _label :!via `Open`))

(event `self.Trigger.OnComponentEndOverlap`
  (params (OverlappedComponent :type "PrimitiveComponent Object Reference") (OtherActor :type "Actor Object Reference") (OtherComp :type "PrimitiveComponent Object Reference") (OtherBodyIndex :type Integer))
  (cast `/Game/FirstPerson/Blueprints/BP_FP_Fae` OtherActor)
  (`self.EnableInput` (`GameplayStatics.GetPlayerController` 0))
  (goto _label :!via `Close`))

(fn `UserConstructionScript`)