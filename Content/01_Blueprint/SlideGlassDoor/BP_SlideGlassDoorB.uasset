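; Sliding glass door that opens for a BP_FP_Fae character carrying both a keycard and a spoon.
; Entering the trigger with both items plays a Timeline whose track drives the relative location of DoorB.
; Leaving the trigger reverses the Timeline to close the door, provided the character still has both items.
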(event `self.Trigger.OnComponentBeginOverlap`
  (params (OverlappedComponent :type "PrimitiveComponent Object Reference") (OtherActor :type "Actor Object Reference") (OtherComp :type "PrimitiveComponent Object Reference") (OtherBodyIndex :type Integer) (bFromSweep :type Boolean) (SweepResult :type "HitResult Structure (by ref)"))
  (bind _asbp_fp_fae (cast `/Game/FirstPerson/Blueprints/BP_FP_Fae` OtherActor))
  (if (and (`/Game/FirstPerson/Blueprints/BP_FP_Fae.HasKeycard?` _asbp_fp_fae) (`/Game/FirstPerson/Blueprints/BP_FP_Fae.HasSpoon?` _asbp_fp_fae))
    (bind (_direction _newtrack_0) (`Timeline|Timeline` :!label _label)
      (:`Update`
        (`SceneComponent.K2_SetRelativeLocationAndRotation` :`self` (`self.DoorB`) :`NewLocation` _newtrack_0)))))

(event `self.Trigger.OnComponentEndOverlap`
  (params (OverlappedComponent :type "PrimitiveComponent Object Reference") (OtherActor :type "Actor Object Reference") (OtherComp :type "PrimitiveComponent Object Reference") (OtherBodyIndex :type Integer))
  (bind _asbp_fp_fae (cast `/Game/FirstPerson/Blueprints/BP_FP_Fae` OtherActor))
  (if (and (`/Game/FirstPerson/Blueprints/BP_FP_Fae.HasKeycard?` _asbp_fp_fae) (`/Game/FirstPerson/Blueprints/BP_FP_Fae.HasSpoon?` _asbp_fp_fae))
    (goto _label :!via `Reverse`)))

(fn `UserConstructionScript`)