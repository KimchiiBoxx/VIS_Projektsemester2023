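; Blockout sliding glass door actor with two door components, DoorA and DoorB, each moved in relative space by its own timeline.
; OpenTriggerA plays DoorA's timeline on overlap and reverses it on exit.
; DoorB's timeline plays on any actor-level overlap rather than OpenTriggerB's, but reverses when OpenTriggerB's overlap ends.
; DoorB also resets its relative transform before each play or reverse.
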(event `self.OpenTriggerA.OnComponentBeginOverlap`
  (params (OverlappedComponent :type "PrimitiveComponent Object Reference") (OtherActor :type "Actor Object Reference") (OtherComp :type "PrimitiveComponent Object Reference") (OtherBodyIndex :type Integer) (bFromSweep :type Boolean) (SweepResult :type "HitResult Structure (by ref)"))
  (bind (_direction _newtrack_0) (`Timeline|TimelineDoorA` :!label _label)
    (:`Update`
      (`SceneComponent.K2_SetRelativeLocationAndRotation` :`self` (`self.DoorA`) :`NewLocation` _newtrack_0))))

(event `self.OpenTriggerA.OnComponentEndOverlap`
  (params (OverlappedComponent :type "PrimitiveComponent Object Reference") (OtherActor :type "Actor Object Reference") (OtherComp :type "PrimitiveComponent Object Reference") (OtherBodyIndex :type Integer))
  (goto _label :!via `Reverse`))

(event `self.ReceiveActorBeginOverlap`
  (params (OtherActor :type "Actor Object Reference"))
  (`SceneComponent.ResetRelativeTransform` (`self.DoorB`))
  (bind (_direction _newtrack_0) (`Timeline|TimelineDoorB` :!label _label_2)
    (:`Update`
      (`SceneComponent.K2_SetRelativeLocationAndRotation` :`self` (`self.DoorB`) :`NewLocation` _newtrack_0))))

(event `self.OpenTriggerB.OnComponentEndOverlap`
  (params (OverlappedComponent :type "PrimitiveComponent Object Reference") (OtherActor :type "Actor Object Reference") (OtherComp :type "PrimitiveComponent Object Reference") (OtherBodyIndex :type Integer))
  (`SceneComponent.ResetRelativeTransform` (`self.DoorB`))
  (goto _label_2 :!via `Reverse`))

(fn `UserConstructionScript`)